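; BP_Player is the player character, handling walking, running and mouse look through Enhanced Input.
; On BeginPlay it adds the PlayerMapping context, puts the WB_MiniMap widget on screen and starts at walk speed.
; Movement follows actor orientation, with run input switching the Speed value passed as AddMovementInput's scale, not a movement component's max speed.
; Mouse X yaws the capsule and mouse Y pitches the camera, scaled by Sense, with no explicit pitch clamp.
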(event Input|EnhancedActionEvents|EnhancedInputActionPlayer_Run
  (params (ActionValue :type Boolean) (ElapsedSeconds :type Float%20%28double-precision%29) (TriggeredSeconds :type Float%20%28double-precision%29) (InputAction :type Input%20Action%20Object%20Reference :default "/Game/Novo_Projeto/Programming/Player/Input/Player_Run.Player_Run"))
  ;[1 1 1] Movement
  (:Triggered
    (Variables|Default|Setspeed (Variables|Default|GetrunSpeed)))
  (:Completed
    (Variables|Default|Setspeed (Variables|Default|GetwalkSpeed))))

(event Input|EnhancedActionEvents|EnhancedInputActionPlayer_Walk
  (params (ActionValue :type Vector%202D%20Structure) (ElapsedSeconds :type Float%20%28double-precision%29) (TriggeredSeconds :type Float%20%28double-precision%29) (InputAction :type Input%20Action%20Object%20Reference :default "/Game/Novo_Projeto/Programming/Player/Input/Player_Walk.Player_Walk"))
  ;[1 1 1] Movement
  (Pawn|Input|AddMovementInput (Math|Transform|TransformDirection (Transformation|GetActorTransform) (Math|Conversions|ToVector(Vector2D) ActionValue)) (Variables|Default|Getspeed) false))

(event Input|EnhancedActionEvents|EnhancedInputActionPlayer_Mouse
  (params (ActionValue :type Vector%202D%20Structure) (ElapsedSeconds :type Float%20%28double-precision%29) (TriggeredSeconds :type Float%20%28double-precision%29) (InputAction :type Input%20Action%20Object%20Reference :default "/Game/Novo_Projeto/Programming/Player/Input/Player_Mouse.Player_Mouse"))
  ;[1 1 1] Camera
  (Utilities|FlowControl|Sequence
    (:then_0
      (Transformation|AddLocalRotation (Variables|Default|GetCapsule) (Math|Rotator|MakeRotator 0.0 0.0 (* (.x ActionValue) (Variables|Default|Getsense))) false false))
    (:then_1
      (Transformation|AddLocalRotation (Variables|Default|GetCamera) (Math|Rotator|MakeRotator 0.0 (* (.y ActionValue) (Variables|Default|Getsense)) 0.0) false false))))

(event EventBeginPlay
  (Utilities|FlowControl|Sequence
    (:then_0
      ;[1 1 1] Enable Inputs
      (Input|AddMappingContext (PlayerController|LocalPlayerSubsystems|GetEnhancedInputLocalPlayerSubsystem (Game|GetPlayerController 0)) "/Game/Novo_Projeto/Programming/Player/Input/PlayerMapping.PlayerMapping" 0 "(bIgnoreAllPressedKeysUntilRelease=True,bForceImmediately=False,bNotifyUserSettings=False)")
      (bind _returnvalue (UserInterface|CreateWidget "/Game/Novo_Projeto/UI/WB_MiniMap.WB_MiniMap_C" (Game|GetPlayerController 0)))
      (UserInterface|Viewport|AddtoViewport _returnvalue 0))
    (:then_1
      ;[1 1 1] Set initial speed
      (Variables|Default|Setspeed (Variables|Default|GetwalkSpeed)))))

(event Collision|EventActorBeginOverlap
  (params (OtherActor :type Actor%20Object%20Reference)))

(event EventTick
  (params (DeltaSeconds :type Float%20%28single-precision%29)))

(fn ConstructionScript)