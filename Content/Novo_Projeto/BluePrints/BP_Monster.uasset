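; BP_Monster is an AI monster with patrol, search and chase behaviors driven by an integer State checked every Tick.
; Patrol runs whenever State is not 1, moving through WalkPoints and wrapping PointCounter to loop the route.
; State 2 issues a search move with no destination set, and state 3 chases the player pawn.
; Nothing here sets the chase state, and MoveToNextPoint is an empty stub.
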(event EventBeginPlay)

(event Collision|EventActorBeginOverlap
  (params (OtherActor :type Actor%20Object%20Reference)))

(event EventTick
  (params (DeltaSeconds :type Float%20%28single-precision%29))
  (Utilities|FlowControl|Sequence
    (:then_0
      ;[1 1 1] Patrol
      (if (not (== (Variables|Default|Getstate) 1))
        (AI|AIMoveTo (Variables|Default|GetaiController) "0, 0, 0" (Utilities|Array|Get(acopy) (Variables|Default|GetwalkPoints) (Variables|Default|GetpointCounter)) -1.0 "Default" "Default" true true
          (:OnMoveFinished
            (Utilities|FlowControl|Sequence
              (:then_0
                (Variables|Default|SetpointCounter (+ 1 (Variables|Default|GetpointCounter))))
              (:then_1
                (if (== (Utilities|Array|Length (Variables|Default|GetwalkPoints)) (Variables|Default|GetpointCounter))
                  (Variables|Default|SetpointCounter 0)))
              (:then_2
                (Variables|Default|Setstate 0)))))))
    (:then_1
      ;[1 1 1] Search
      (if (== (Variables|Default|Getstate) 2)
        (AI|AIMoveTo (Variables|Default|GetaiController) "0, 0, 0" 0 -1.0 "Default" "Default" true true
          (:then
            (Variables|Default|Setstate 0))
          (:OnMoveFinished
            (Variables|Default|Setstate 1)))))
    (:then_2
      ;[1 1 1] Chase
      (if (== (Variables|Default|Getstate) 3)
        (AI|AIMoveTo (Variables|Default|GetaiController) "0, 0, 0" (Game|Player|GetPlayerPawn 0) -1.0 "Default" "Default" true true)))))

(fn ConstructionScript)

(fn MovetoNextPoint)