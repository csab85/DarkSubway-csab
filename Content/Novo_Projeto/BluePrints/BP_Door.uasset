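; BP_Door is an interactable door that the player swings open with the E key unless it is Locked.
; InteractTrigger overlaps with BP_Player enable and disable the door's input, so E only works nearby.
; DoorOpenTimeline rotates the whole actor's yaw toward 90 degrees from its BeginPlay yaw, signed by OpenDIrection.
; The lerp starts from the current yaw each update, compounding the easing, and no closing logic exists.
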(event OnComponentBeginOverlap(InteractTrigger)
  (params (OverlappedComponent :type Primitive%20Component%20Object%20Reference) (OtherActor :type Actor%20Object%20Reference) (OtherComp :type Primitive%20Component%20Object%20Reference) (OtherBodyIndex :type Integer) (bFromSweep :type Boolean) (SweepResult :type Hit%20Result%20Structure%20%28by%20ref%29))
  ;[1 1 1] Enable/Disable interaction
  (Utilities|Casting|CastToBP_Player OtherActor)
  (Input|EnableInput (Game|GetPlayerController 0)))

(event OnComponentEndOverlap(InteractTrigger)
  (params (OverlappedComponent :type Primitive%20Component%20Object%20Reference) (OtherActor :type Actor%20Object%20Reference) (OtherComp :type Primitive%20Component%20Object%20Reference) (OtherBodyIndex :type Integer))
  ;[1 1 1] Enable/Disable interaction
  (Utilities|Casting|CastToBP_Player OtherActor)
  (Input|DisableInput (Game|GetPlayerController 0)))

(event EventBeginPlay
  (Variables|Default|SetinitialYaw (.yaw (Transformation|GetActorRotation))))

(event Collision|EventActorBeginOverlap
  (params (OtherActor :type Actor%20Object%20Reference)))

(event EventTick
  (params (DeltaSeconds :type Float%20%28single-precision%29)))

(event Input|KeyboardEvents|E
  (params (Key :type Key%20Structure :default "None"))
  (bind _returnvalue (Transformation|GetActorRotation))
  ;[1 1 1] Open Door
  (:Pressed
    (if (not (Variables|Default|Getlocked))
      (bind _rotation (Timeline|Door%20Open%20Timeline Play)
        (:Update
          (Transformation|SetActorRotation (Math|Rotator|MakeRotator (.roll _returnvalue) (.pitch _returnvalue) (Math|Float|Lerp (.yaw (Transformation|GetActorRotation)) (+ (Variables|Default|GetinitialYaw) (* 9e+01 (Variables|Default|GetopenDIrection))) _rotation))))))))

(fn ConstructionScript)