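; BP_PlayerNew is the player character, with Enhanced Input walking, running and mouse look using clamped camera pitch.
; Running swaps the speed value that scales movement input.
; Probing plays a timeline animating the map cover sprite's alpha, blocks retriggering until finished, and switches the BP_Monster found at BeginPlay to state 2.
; Tick polls the piece count and, at three, finds the Metro actor and enables level passing.
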(event Input|EnhancedActionEvents|EnhancedInputActionPlayer_Run
  (params (ActionValue :type Boolean) (ElapsedSeconds :type Float%20%28double-precision%29) (TriggeredSeconds :type Float%20%28double-precision%29) (InputAction :type Input%20Action%20Object%20Reference :default "/Game/Novo_Projeto/Input/Player_Run.Player_Run"))
  ;[1 1 1] Movement
  (:Triggered
    (Variables|Default|Setspeed (Variables|Default|GetrunSpeed)))
  (:Completed
    (Variables|Default|Setspeed (Variables|Default|GetwalkSpeed))))

(event Input|EnhancedActionEvents|EnhancedInputActionPlayer_Walk
  (params (ActionValue :type Vector%202D%20Structure) (ElapsedSeconds :type Float%20%28double-precision%29) (TriggeredSeconds :type Float%20%28double-precision%29) (InputAction :type Input%20Action%20Object%20Reference :default "/Game/Novo_Projeto/Input/Player_Walk.Player_Walk"))
  ;[1 1 1] Movement
  (Pawn|Input|AddMovementInput (Math|Transform|TransformDirection (Transformation|GetActorTransform) (Math|Conversions|ToVector(Vector2D) ActionValue)) (Variables|Default|Getspeed) false))

(event Input|EnhancedActionEvents|EnhancedInputActionPlayer_Mouse
  (params (ActionValue :type Vector%202D%20Structure) (ElapsedSeconds :type Float%20%28double-precision%29) (TriggeredSeconds :type Float%20%28double-precision%29) (InputAction :type Input%20Action%20Object%20Reference :default "/Game/Novo_Projeto/Input/Player_Mouse.Player_Mouse"))
  ;[1 1 1] Camera
  (Utilities|FlowControl|Sequence
    (:then_0
      (Pawn|Input|AddControllerYawInput (* (* (.x ActionValue) (Variables|Default|Getsense)) 0.5)))
    (:then_1
      (bind _output_get (Variables|Default|SetcameraPitch (+ (* (.y ActionValue) (Variables|Default|Getsense)) (Variables|Default|GetcameraPitch))))
      (bind _output_get_2 (Variables|Default|SetcameraPitch (Math|Float|Clamp(Float) _output_get (Variables|Default|GetminPitch) (Variables|Default|GetmaxPitch))))
      (Transformation|SetWorldRotation (Variables|Default|GetCamera) (Math|Rotator|MakeRotator 0.0 _output_get_2 (.yaw (Transformation|GetWorldRotation (Variables|Collision|GetCapsuleComponent)))) false false))))

(event Input|EnhancedActionEvents|EnhancedInputActionPlayer_Probe
  (params (ActionValue :type Boolean) (ElapsedSeconds :type Float%20%28double-precision%29) (TriggeredSeconds :type Float%20%28double-precision%29) (InputAction :type Input%20Action%20Object%20Reference :default "/Game/Novo_Projeto/Input/Player_Probe.Player_Probe"))
  (bind _coverinitialcolor (Variables|Default|GetcoverInitialColor))
  ;[1 1 1] Probe
  (if (not (Variables|Default|Getprobing))
    (Utilities|FlowControl|Sequence
      (:then_0
        (Variables|Default|Setprobing true)
        (bind _alpha_track (Timeline|Timeline PlayFromStart)
          (:Update
            (Sprite|SetSpriteColor (Variables|Default|GetMap%20Cover) (Utilities|Struct|MakeLinearColor (Math|Conversions|ToFloat(Byte) (.r _coverinitialcolor)) (Math|Conversions|ToFloat(Byte) (.g _coverinitialcolor)) (Math|Conversions|ToFloat(Byte) (.b _coverinitialcolor)) (Math|Float|Lerp 0.0 1.0 _alpha_track))))
          (:Finished
            (Variables|Default|Setprobing false))))
      (:then_1
        (bind _asbp_monster (Utilities|Casting|CastToBP_Monster (Variables|Default|Getmonster)))
        (Variables|/Game/Novo_Projeto/BluePrints/BP_Monster.BP_Monster_C|Setstate _asbp_monster 2)))))

(event EventBeginPlay
  (Utilities|FlowControl|Sequence
    (:then_0
      ;[1 1 1] Enable Inputs
      (Input|AddMappingContext (PlayerController|LocalPlayerSubsystems|GetEnhancedInputLocalPlayerSubsystem (Game|GetPlayerController 0)) "/Game/Novo_Projeto/Input/PlayerMapping.PlayerMapping" 0 "(bIgnoreAllPressedKeysUntilRelease=True,bForceImmediately=False,bNotifyUserSettings=False)"))
    (:then_1
      ;[1 1 1] Set initial speed
      (Variables|Default|Setspeed (Variables|Default|GetwalkSpeed)))
    (:then_2
      ;[1 1 1] Set monster
      (bind _returnvalue (Actor|GetActorOfClass "/Game/Novo_Projeto/BluePrints/BP_Monster.BP_Monster_C"))
      (Variables|Default|Setmonster _returnvalue))))

(event Collision|EventActorBeginOverlap
  (params (OtherActor :type Actor%20Object%20Reference)))

(event EventTick
  (params (DeltaSeconds :type Float%20%28single-precision%29))
  ;[1 1 1] Check if can pass level
  (if (== (Variables|Default|Getpieces) 3)
    (bind _returnvalue (Actor|GetActorOfClass "/Game/Blue/Metro.Metro_C"))
    (bind _asmetro (Utilities|Casting|CastToMetro _returnvalue))
    (Variables|/Game/Blue/Metro.Metro_C|Setpasslevel _asmetro true)))

(fn ConstructionScript)